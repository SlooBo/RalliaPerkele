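; HUD that provides mouse edge scrolling by driving the forward and right edge axes on the owning Pawn_EdgeScrolling.
; DrawHUD lays eight input-consuming hit boxes along the screen's edges and corners, with optional debug-style color overlays.
; Each box encodes type, ID and index in its dotted name, which cursor-over events parse to set the pawn's axes.
; Corners set both axes, and leaving an edge box zeroes them.
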(event EventBeginPlay
  (bind _aspawn_edgescrolling_c (Utilities|Casting|CastToPawn_EdgeScrolling (Class|HUD|GetOwningPawn)))
  (Variables|Default|SetOwningPawn _aspawn_edgescrolling_c))

(event EventHitBoxBeginCursorOver
  (params (BoxName :type Name :default "None"))
  (bind _element_id_s (Utilities|GetHitBoxType (Utilities|Text|ToText(Name) BoxName))
    (:EdgeBox
      (Utilities|EdgeBoxEvents _element_id_s
        (:TopLeft
          (Utilities|EdgeMovement :!label _label))
        (:TopMid
          (goto _label TopMiddle))
        (:TopRight
          (goto _label TopRight))
        (:MiddleRIght
          (goto _label MiddleRight))
        (:BottomRight
          (goto _label BottomRight))
        (:BottomMiddle
          (goto _label BottomMiddle))
        (:BottomLeft
          (goto _label BottomLeft))
        (:MiddleLeft
          (goto _label MiddleLeft))))))

(event EventHitBoxEndCursorOver
  (params (BoxName :type Name :default "None"))
  (bind _element_id_s (Utilities|GetHitBoxType (Utilities|Text|ToText(Name) BoxName))
    (:EdgeBox
      (Utilities|EdgeBoxEvents _element_id_s
        (:TopLeft
          _)
        (:TopMid
          _)
        (:TopRight
          _)
        (:MiddleRIght
          _)
        (:BottomRight
          _)
        (:BottomMiddle
          _)
        (:BottomLeft
          _)
        (:MiddleLeft
          _))
      (CallFunction|ResetEdgeMovement))))

(event EventDrawHUD
  (params (SizeX :type Integer) (SizeY :type Integer))
  (bind _returnvalue (Math|Conversions|ToFloat(Integer) SizeX))
  (bind _returnvalue_2 (Math|Conversions|ToFloat(Integer) SizeY))
  (bind _returnvalue_3 (Math|Vector2D|MakeVector2D _returnvalue _returnvalue_2))
  (Variables|Default|SetScreenResolution _returnvalue_3)
  (CallFunction|DrawEdgeHitBoxes :Size _returnvalue_3 :EdgeThickness 64.0 :OverLayColor "(R=0.937255,G=0.000000,B=0.406979,A=1.000000)" :bConsumeInput? true))

(fn ConstructionScript)

(fn DrawHitBoxwithOverLay
  (params (position :type Vector%202D%20Structure) (Size :type Vector%202D%20Structure) (Name :type Name) (bConsumeInput :type Boolean) (Priority :type Integer) (bShowOverlay? :type Boolean) (OverLayColor :type Linear%20Color%20Structure))
  (bind (_x _y) (Math|Vector2D|BreakVector2D Size))
  (bind (_x_2 _y_2) (Math|Vector2D|BreakVector2D position))
  (Class|HUD|AddHitBox position Size Name bConsumeInput Priority)
  (if bShowOverlay?
    (HUD|DrawRect OverLayColor _x_2 _y_2 _x _y)))

(fn DrawEdgeHitBoxes
  (params (ID :type Integer) (Location :type Vector%202D%20Structure) (Size :type Vector%202D%20Structure) (EdgeThickness :type Float%20%28single-precision%29) (bShowOverlays? :type Boolean) (OverLayColor :type Linear%20Color%20Structure) (bConsumeInput? :type Boolean) (Priority :type Integer))
  (LocalVariables|SetL_ID ID)
  (LocalVariables|SetL_Location Location)
  (LocalVariables|SetL_Size Size)
  (LocalVariables|SetL_EdgeThickness EdgeThickness)
  (LocalVariables|SetL_ShowOverLays? bShowOverlays?)
  (LocalVariables|SetL_OverlayColor OverLayColor)
  (LocalVariables|SetL_ConsumeInput? bConsumeInput?)
  (LocalVariables|SetL_Priority Priority)
  (for _index (range 0 7)
    (CallFunction|DrawHitBoxwithOverLay (Utilities|Select :Index _index :Option%200 (.TopLeft (Utilities|Get8LocationforEdges (LocalVariables|GetL_Location) (LocalVariables|GetL_Size) (LocalVariables|GetL_EdgeThickness))) :Option%201 (.TopMiddle (Utilities|Get8LocationforEdges (LocalVariables|GetL_Location) (LocalVariables|GetL_Size) (LocalVariables|GetL_EdgeThickness))) :Option%202 (.TopRight (Utilities|Get8LocationforEdges (LocalVariables|GetL_Location) (LocalVariables|GetL_Size) (LocalVariables|GetL_EdgeThickness))) :Option%203 (.MiddleRight (Utilities|Get8LocationforEdges (LocalVariables|GetL_Location) (LocalVariables|GetL_Size) (LocalVariables|GetL_EdgeThickness))) :Option%204 (.BottomRight (Utilities|Get8LocationforEdges (LocalVariables|GetL_Location) (LocalVariables|GetL_Size) (LocalVariables|GetL_EdgeThickness))) :Option%205 (.BottomMiddle (Utilities|Get8LocationforEdges (LocalVariables|GetL_Location) (LocalVariables|GetL_Size) (LocalVariables|GetL_EdgeThickness))) :Option%206 (.BottomLeft (Utilities|Get8LocationforEdges (LocalVariables|GetL_Location) (LocalVariables|GetL_Size) (LocalVariables|GetL_EdgeThickness))) :Option%207 (.MiddleLeft (Utilities|Get8LocationforEdges (LocalVariables|GetL_Location) (LocalVariables|GetL_Size) (LocalVariables|GetL_EdgeThickness)))) (Utilities|Select :Index _index :Option%200 (Math|Vector2D|MakeVector2D (LocalVariables|GetL_EdgeThickness) (LocalVariables|GetL_EdgeThickness)) :Option%201 (.XLength (Utilities|CreateEdgeHitboxSizes (LocalVariables|GetL_Size) (LocalVariables|GetL_EdgeThickness))) :Option%202 (Math|Vector2D|MakeVector2D (LocalVariables|GetL_EdgeThickness) (LocalVariables|GetL_EdgeThickness)) :Option%203 (.YLength (Utilities|CreateEdgeHitboxSizes (LocalVariables|GetL_Size) (LocalVariables|GetL_EdgeThickness))) :Option%204 (Math|Vector2D|MakeVector2D (LocalVariables|GetL_EdgeThickness) (LocalVariables|GetL_EdgeThickness)) :Option%205 (.XLength (Utilities|CreateEdgeHitboxSizes (LocalVariables|GetL_Size) (LocalVariables|GetL_EdgeThickness))) :Option%206 (Math|Vector2D|MakeVector2D (LocalVariables|GetL_EdgeThickness) (LocalVariables|GetL_EdgeThickness)) :Option%207 (.YLength (Utilities|CreateEdgeHitboxSizes (LocalVariables|GetL_Size) (LocalVariables|GetL_EdgeThickness)))) (Utilities|CreateHitBoxName "EdgeBox" (LocalVariables|GetL_ID) _index) (LocalVariables|GetL_ConsumeInput?) (LocalVariables|GetL_Priority) (LocalVariables|GetL_ShowOverLays?) (LocalVariables|GetL_OverlayColor))))

(fn ResetEdgeMovement
  (bind _owningpawn (Variables|Default|GetOwningPawn))
  (Variables|/Game/Blueprints/Pawn_EdgeScrolling.Pawn_EdgeScrolling_C|SetEdgeForwardAxis _owningpawn 0.0)
  (Variables|/Game/Blueprints/Pawn_EdgeScrolling.Pawn_EdgeScrolling_C|SetEdgeRightAxis _owningpawn 0.0))