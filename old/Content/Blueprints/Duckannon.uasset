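; Duckannon is a projectile actor that damages Sedan vehicles.
; On its first Tick, a one-shot flag lets it add a large forward velocity to its physics-driven static mesh.
; An overlap or hit destroys it and prints a debug message, and a hit on a Sedan also subtracts fixed Health and prints the new value.
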(event `self.ReceiveActorBeginOverlap`
  (params (OtherActor :type "Actor Object Reference"))
  (`self.K2_DestroyActor` :!label _label)
  (`KismetSystemLibrary.PrintString` null "osuma"))

(event `self.ReceiveTick`
  (params (DeltaSeconds :type "Float (single-precision)"))
  (if (not (`self.Paskafix`))
    (`PrimitiveComponent.SetPhysicsLinearVelocity` (`self.StaticMesh1`) (* (`self.GetActorForwardVector`) 10000.0) true "None")
    (set `self.Paskafix` true)))

(event `self.ReceiveHit`
  (params (MyComp :type "PrimitiveComponent Object Reference") (Other :type "Actor Object Reference") (OtherComp :type "PrimitiveComponent Object Reference") (bSelfMoved :type Boolean) (HitLocation :type "Object.Vector Structure") (HitNormal :type "Object.Vector Structure") (NormalImpulse :type "Object.Vector Structure") (Hit :type "EngineTypes.HitResult Structure (by ref)"))
  (`|ExecutionSequence`
    (:`then_0`
      (goto _label))
    (:`then_1`
      (bind _assedan_c (cast `/Game/Sedan/Sedan` Other))
      (set `/Game/Sedan/Sedan.Health` (+ (`/Game/Sedan/Sedan.Health` _assedan_c) -10) _assedan_c)
      (`KismetSystemLibrary.PrintString` (`KismetStringLibrary.Conv_IntToString` (`/Game/Sedan/Sedan.Health` _assedan_c))))))

(fn `UserConstructionScript`
  (set `self.Paskafix` false))