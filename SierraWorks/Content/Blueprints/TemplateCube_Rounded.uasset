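; TemplateCube_Rounded is an actor that turns to face the first player's pawn horizontally.
; Every Tick it derives a yaw from the direction vector to the pawn and applies it, keeping its current pitch and roll.
; A look-at pitch calculation is left unconnected, and the construction script is empty.
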(event `self.ReceiveTick`
  (params (DeltaSeconds :type "Float (single-precision)"))
  (`self.SetActorRotation` (`KismetMathLibrary.MakeRot` (.pitch (`self.K2_GetActorRotation`)) (.yaw (`KismetMathLibrary.Conv_VectorToRotator` (- (`self.K2_GetActorLocation` (`GameplayStatics.GetPlayerPawn` 0)) (`self.K2_GetActorLocation`)))) (.roll (`self.K2_GetActorRotation`)))))

(fn `UserConstructionScript`)