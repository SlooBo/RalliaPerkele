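; Strategy-style camera pawn with wheel zoom, hold-to-rotate orbit and planar panning.
; Camera1 sits on a sphere around the pawn origin, positioned by clamped radius, yaw and height angles and always looking at the center, also applied in the construction script.
; Movement follows the camera's yaw only, adding edge-scroll axis values to input.
; Those edge values are read here but never set.
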(event `InputAction|WheelMouseUP`
  (:`Pressed`
    (set `self.Camera Radius` (`KismetMathLibrary.FClamp` (- (`self.Camera Radius`) (`self.ZoomSPeed`)) (`self.RadiusMin`) (`self.RadiusMax`)))
    (`self.UpdateCameraLocation&Rotation` :!label _label)))

(event `InputAction|WheelMouseDown`
  (:`Pressed`
    (set `self.Camera Radius` (`KismetMathLibrary.FClamp` (+ (`self.Camera Radius`) (`self.ZoomSPeed`)) (`self.RadiusMin`) (`self.RadiusMax`)))
    (goto _label)))

(event `InputAction|RotateCamera`
  (:`Pressed`
    (set `self.bRotateCamera?` true))
  (:`Released`
    (set `self.bRotateCamera?` false)))

(event `InputAxis|MouseX`
  (params (AxisValue :type "Float (single-precision)"))
  (if (`self.bRotateCamera?`)
    (set `self.Camera ZAngle` (+ (* AxisValue (`self.RotateSpeed`)) (`self.Camera ZAngle`)))
    (`self.UpdateCameraLocation&Rotation` :!label _label_2)))

(event `InputAxis|MouseY`
  (params (AxisValue :type "Float (single-precision)"))
  (if (`self.bRotateCamera?`)
    (set `self.Camera Height Angle` (`KismetMathLibrary.FClamp` (+ (* AxisValue (`self.RotateSpeed`)) (`self.Camera Height Angle`)) 10.0 90.0))
    (goto _label_2)))

(event `InputAxis|MoveForward`
  (params (AxisValue :type "Float (single-precision)"))
  (`self.K2_SetActorLocation` (`self.AddVectorLocation` (`KismetMathLibrary.GetForwardVector` (`self.IsolateYaw` (`SceneComponent.K2_GetComponentRotation` (`self.Camera1`)))) (* (+ AxisValue (`self.EdgeForwardAxis`)) (`self.MovementSpeed`)))))

(event `InputAxis|MoveRight`
  (params (AxisValue :type "Float (single-precision)"))
  (`self.K2_SetActorLocation` (`self.AddVectorLocation` (`KismetMathLibrary.GetRightVector` (`self.IsolateYaw` (`SceneComponent.K2_GetComponentRotation` (`self.Camera1`)))) (* (+ AxisValue (`self.EdgeRightAxis`)) (`self.MovementSpeed`)))))

(fn `UpdateCameraLocation&Rotation`
  (`SceneComponent.SetRelativeLocation` (`self.Camera1`) (`.Location` (`self.PointOnASphere` (`self.Camera Radius`) (`self.Camera ZAngle`) (`self.Camera Height Angle`))) false)
  (`SceneComponent.SetRelativeRotation` (`self.Camera1`) (`KismetMathLibrary.FindLookAtRotation` (`SceneComponent.RelativeLocation` (`self.Camera1`)) (`KismetMathLibrary.MakeVector` 0.0)) false))

(fn `UserConstructionScript`
  (`self.UpdateCameraLocation&Rotation`))