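; Menu is a hit-driven option selector that cycles three configurable labels on a text render and saves the choice, apparently for customizing Wheels, Sides or Body parts.
; The construction script fills the label array from three Selection variables and displays the first.
; Each mesh hit advances the label, then loads or creates an OptionsSave in "saveFile".
; CheckPlace maps the label's prefix to the save array slot to overwrite.
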(event OnComponentHit(StaticMesh1)
  (params (OtherActor :type Actor%20Object%20Reference) (OtherComp :type Primitive%20Component%20Object%20Reference) (NormalImpulse :type Vector :default "0, 0, 0") (Hit :type Hit%20Result%20Structure%20%28by%20ref%29))
  (bind _svsubclass (Variables|Default|GetSvSubClass))
  (bind _svsubclass_2 (Variables|Default|GetSvSubClass))
  (Variables|Default|Seti (+ (Variables|Default|Geti) 1))
  (Math|Integer|CompareInt (Variables|Default|Geti) 2
    (:>
      (Variables|Default|Seti 0))
    (:==
      _)
    (:<
      _))
  (Rendering|Components|TextRender|SetText (Variables|Default|GetTextRender1) (Utilities|Array|Get(acopy) (Variables|Default|GetStringArray) (Variables|Default|Geti)))
  (bind _returnvalue (SaveGame|DoesSaveGameExist "saveFile"))
  (if _returnvalue
    (bind _returnvalue_2 (SaveGame|LoadGamefromSlot "saveFile"))
    (Variables|Default|SetsvSubClass _returnvalue_2)
    (bind _asoptionssave_c (Utilities|Casting|CastToOptionsSave _svsubclass_2))
    (bind _index (CallFunction|CheckPlace (Utilities|Array|Get(acopy) (Variables|Default|GetStringArray) (Variables|Default|Geti))))
    (Utilities|Array|SetArrayElem (Variables|/Game/Blueprints/OptionsSave.OptionsSave_C|GetLocallySavedStrings _asoptionssave_c) _index (Utilities|Array|Get(acopy) (Variables|Default|GetStringArray) (Variables|Default|Geti)) true)
    (SaveGame|SaveGametoSlot _svsubclass_2 "saveFile")
    (Development|PrintString (Utilities|Array|Get(acopy) (Variables|/Game/Blueprints/OptionsSave.OptionsSave_C|GetLocallySavedStrings _asoptionssave_c) _index))
    (else
      (bind _returnvalue_3 (SaveGame|CreateSaveGameObject "/Game/Blueprints/OptionsSave.OptionsSave_C"))
      (Variables|Default|SetsvSubClass _returnvalue_3)
      (bind _asoptionssave_c_2 (Utilities|Casting|CastToOptionsSave _svsubclass))
      (bind _index_2 (CallFunction|CheckPlace (Utilities|Array|Get(acopy) (Variables|Default|GetStringArray) (Variables|Default|Geti))))
      (Utilities|Array|SetArrayElem (Variables|/Game/Blueprints/OptionsSave.OptionsSave_C|GetLocallySavedStrings _asoptionssave_c_2) _index_2 (Utilities|Array|Get(acopy) (Variables|Default|GetStringArray) (Variables|Default|Geti)) true)
      (SaveGame|SaveGametoSlot _svsubclass "saveFile")
      (Development|PrintString (Utilities|Array|Get(acopy) (Variables|/Game/Blueprints/OptionsSave.OptionsSave_C|GetLocallySavedStrings _asoptionssave_c_2) _index_2)))))

(fn ConstructionScript
  (bind _selection (Variables|Default|GetSelection))
  (bind _stringarray (Variables|Default|GetStringArray))
  (Utilities|Array|SetArrayElem _stringarray 0 _selection true)
  (Utilities|Array|SetArrayElem _stringarray 1 (Variables|Default|GetSelection2) true)
  (Utilities|Array|SetArrayElem _stringarray 2 (Variables|Default|GetSelection3) true)
  (Rendering|Components|TextRender|SetText (Variables|Default|GetTextRender1) _selection))

(fn CheckPlace
  (params (Input%20String :type String))
  (if (Utilities|String|StartsWith Input%20String "Wheels")
    (LocalVariables|SetReturn%20index 0)
    (Development|PrintString (Utilities|String|ToString(Integer) (LocalVariables|GetReturn%20index)) :!label _label)
    (return (LocalVariables|GetReturn%20index))
    (elif (Utilities|String|StartsWith Input%20String "Sides")
      (LocalVariables|SetReturn%20index 1)
      (goto _label)
      (elif (Utilities|String|StartsWith Input%20String "Body")
        (LocalVariables|SetReturn%20index 2)
        (goto _label)))))